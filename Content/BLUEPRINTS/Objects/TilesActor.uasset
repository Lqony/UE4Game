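; Tile actor whose surface can be switched between stone and wood materials.
; SetMaterial stores the choice, resolves it through GiveMaterial (wood by default) and applies a dynamic instance to the mesh's first slot.
; It sets the U and V texture scale parameters from half the Box's world X and Z scale, so tiling follows the actor's size.
; The event graph and construction script are empty, so SetMaterial must be called externally.
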(event EventBeginPlay)

(event Collision|EventActorBeginOverlap
  (params (OtherActor :type Actor%20Object%20Reference)))

(fn ConstructionScript)

(fn GiveMaterial
  (switch int (Variables|Default|GetMaterial)
    (:Default
      (return "/Game/ASSETS/Map/Tiles/M_WoodTile.M_WoodTile"))
    (:0
      (return "/Game/ASSETS/Map/Tiles/M_StoneTIle.M_StoneTIle"))
    (:1
      (return "/Game/ASSETS/Map/Tiles/M_WoodTile.M_WoodTile"))))

(fn SetMaterial
  (params (_Material :type Integer))
  (bind _box (Variables|Default|GetBox))
  (bind _creaturemesh (Variables|Default|GetCreatureMesh))
  (bind _returnvalue (Transformation|GetWorldScale _box))
  (bind (_x _y _z) (Math|Vector|BreakVector _returnvalue))
  (Variables|Default|SetMaterial _Material)
  (bind _returnvalue_2 (Rendering|Material|CreateDynamicMaterialInstance _creaturemesh 0 (CallFunction|GiveMaterial) :!class /Script/Engine.PrimitiveComponent))
  (Rendering|Material|SetMaterial _creaturemesh 0 _returnvalue_2)
  (bind _output_get (Variables|Default|SetDynamicMatInst _returnvalue_2))
  (Rendering|Material|SetScalarParameterValue _output_get "TextureScaleU" (/ _x 2.0) :!class /Script/Engine.MaterialInstanceDynamic)
  (Rendering|Material|SetScalarParameterValue (Variables|Default|GetDynamicMatInst) "TextureScaleV" (/ _z 2.0) :!class /Script/Engine.MaterialInstanceDynamic))