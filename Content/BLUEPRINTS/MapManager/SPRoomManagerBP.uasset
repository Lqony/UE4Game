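; Room manager Blueprint that triggers room creation and spawns the tile actors attached to it.
; Tick watches a one-shot boolean that, when set, clears itself and calls CreateRoom for room 0.
; SpawnTiles spawns the requested number of TilesActor instances at the manager's transform, always spawning despite collisions, attaches each to the manager and returns them as an array.
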(event EventBeginPlay)

(event Collision|EventActorBeginOverlap
  (params (OtherActor :type Actor%20Object%20Reference)))

(event EventTick
  (params (DeltaSeconds :type Float%20%28single-precision%29))
  (|CallParentFunction DeltaSeconds)
  (if (Variables|RoomManager|GetCreateRoom_0)
    (Variables|RoomManager|SetCreateRoom_0 false)
    (Class|SPRoomManagerCPP|CreateRoom)))

(fn ConstructionScript)

(fn SpawnTiles
  (params (amount :type Integer))
  (for _index (range 1 amount)
    (bind _returnvalue (Game|SpawnActorfromClass "/Game/ASSETS/Map/Tiles/TilesActor.TilesActor_C" (Transformation|GetActorTransform) "AlwaysSpawn" 0 0))
    (Transformation|AttachActorToActor _returnvalue self "None" "KeepRelative" "KeepRelative" "KeepRelative" true)
    (Utilities|Array|Add (LocalVariables|GetOutput) _returnvalue))
  (return (LocalVariables|GetOutput)))