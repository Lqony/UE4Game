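; SPMapManagerBP is a map manager actor with helper functions for streaming in a level and finding room activators.
; CallLoadLevelInstance loads the "Arena2" level as an instance at the world origin, then flags it visible, loaded and blocking on load before returning it.
; GetActivators returns every SPRoomActivatorBP actor in the world, while the event graph and construction script are empty.
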(event EventBeginPlay)

(event Collision|EventActorBeginOverlap
  (params (OtherActor :type Actor%20Object%20Reference)))

(event EventTick
  (params (DeltaSeconds :type Float%20%28single-precision%29)))

(fn ConstructionScript)

(fn CallLoadLevelInstance
  (bind (_boutsuccess _returnvalue) (Class|LevelStreamingKismet|LoadLevelInstance "Arena2" (Math|Vector|MakeVector 0.0 0.0 0.0) (Math|Rotator|MakeRotator 0.0 0.0 0.0)))
  (if _boutsuccess
    (Variables|/Script/Engine.LevelStreaming|SetbShouldBeVisible _returnvalue true)
    (Variables|/Script/Engine.LevelStreaming|SetbShouldBeLoaded _returnvalue true)
    (Variables|/Script/Engine.LevelStreaming|SetbShouldBlockOnLoad _returnvalue true)
    (return _returnvalue)
    (else
      (return 0))))

(fn GetActivators
  (bind _outactors (Actor|GetAllActorsOfClass "/Game/BLUEPRINTS/MapManager/SPRoomActivatorBP.SPRoomActivatorBP_C"))
  (return _outactors))