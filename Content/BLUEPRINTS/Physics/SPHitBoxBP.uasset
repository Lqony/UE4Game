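; Sphere hit box actor that deals hitstun, damage and knockback to overlapped SPPawnCPP pawns while active, respecting owner and friendly-fire rules.
; GetHit runs only on authority; both network branches share the single-hit follow-up, which explodes missiles or destroys the box, then slows time on owner and victim by vertical force.
; Tick draws a red or green debug circle for active state, and show/hide events toggle the Animation component.
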(event Collision|EventActorBeginOverlap
  (params (OtherActor :type Actor%20Object%20Reference))
  (bind _details (Variables|Default|GetDetails))
  (bind (_position _force _activationtime _destroytime _friendlyfire _multihit _owner _damage _hitstun) (Utilities|Struct|BreakSPHitBoxDetails _details))
  (bind _z (Math|Vector|BreakVector _force))
  ;[1 1 1] OVERLAP
  (if (Utilities|Struct|BreakSPHitBoxWorkData (Variables|Default|GetWorkData))
    (if (or _friendlyfire (!= _owner OtherActor))
      (Networking|SwitchHasAuthority
        (:Authority
          (bind _assppawn_cpp (Utilities|Casting|CastToSPPawnCPP OtherActor))
          (Class|SPPawnCPP|GetHit _assppawn_cpp _hitstun _damage _force))
        (:Remote
          _))
      (if (not _multihit)
        (if (.Missile (Utilities|Struct|BreakSPMissileDetails (Variables|Default|GetMissileDetails)))
          (Class|SPHitBoxCPP|ExplodeonHit)
          (else
            (Class|SPHitBoxCPP|DestroyHitBox)))
        (Class|SPPawnCPP|SlowTimebyForce _owner _z)
        (Class|SPPawnCPP|SlowTimebyForce _assppawn_cpp _z)))))

(event EventShowAnimation
  ;[1 1 1] SHOW ANIMATION
  (|CallParentFunction)
  (Rendering|SetVisibility (Variables|Default|GetAnimation) true true))

(event EventTick
  (params (DeltaSeconds :type Float%20%28single-precision%29))
  (bind _returnvalue (Transformation|GetActorLocation))
  (bind _mainbody (Variables|Default|GetMainBody))
  (bind _sphereradius (Variables|/Script/Engine.SphereComponent|GetSphereRadius _mainbody))
  ;[1 1 1] TICK
  (|CallParentFunction DeltaSeconds)
  (Networking|SwitchHasAuthority
    (:Authority
      _)
    (:Remote
      _))
  (if (Utilities|Struct|BreakSPHitBoxWorkData (Variables|Default|GetWorkData))
    (Rendering|Debug|DrawDebugCircle _returnvalue _sphereradius 45 "(R=1.000000,G=0.027806,B=0.000000,A=1.000000)" 0.0 0.0 "1.000000,0.000000,0.000000" "0.000000,0.000000,1.000000")
    (else
      (Rendering|Debug|DrawDebugCircle _returnvalue _sphereradius 45 "(R=0.000000,G=1.000000,B=0.136468,A=1.000000)" 0.0 0.0 "1.000000,0.000000,0.000000" "0.000000,0.000000,1.000000"))))

(event EventHideAnimation
  ;[1 1 1] HIDE ANIMATION
  (|CallParentFunction)
  (Rendering|SetVisibility (Variables|Default|GetAnimation) false true))

(fn ConstructionScript)