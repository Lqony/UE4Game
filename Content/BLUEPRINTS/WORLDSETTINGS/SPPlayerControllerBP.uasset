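; Player controller that feeds gamepad and touch-joystick setup into an SPPawnCPP pawn, cached on BeginPlay and re-fetched on Tick whenever invalid.
; Left-stick axes become directional key flags, with a stronger "Super" tier for hard horizontal pushes; attack, defence and jump setters are unwired.
; Escape and Android Back open the HUD exit menu.
; NativeSpawnSPPawnBP spawns a NinjaPawn on authority only, with its Server flag currently making no difference.
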(event EventBeginPlay
  ;[1 1 1] BEGIN PLAY
  (|CallParentFunction)
  (Networking|SwitchHasAuthority
    (:Authority
      _)
    (:Remote
      _))
  (Class|PlayerController|ActivateTouchInterface (Game|GetPlayerController 0) "/Game/BLUEPRINTS/HUD/PlayerControll/LeftVirtualJoystickOnly.LeftVirtualJoystickOnly")
  (bind _assppawn_cpp (Utilities|Casting|CastToSPPawnCPP (Pawn|GetControlledPawn)))
  (Variables|Default|SetPlayerPawn _assppawn_cpp))

(event EventTick
  (params (DeltaSeconds :type Float%20%28single-precision%29))
  ;[1 1 1] TICK
  (|CallParentFunction DeltaSeconds)
  (if (not (Utilities|IsValid (Variables|Default|GetPlayerPawn)))
    (bind _assppawn_cpp (Utilities|Casting|CastToSPPawnCPP (Pawn|GetControlledPawn)))
    (Variables|Default|SetPlayerPawn _assppawn_cpp)))

(event Input|GamepadEvents|GamepadLeftX
  (params (AxisValue :type Float%20%28single-precision%29))
  (bind _playerpawn (Variables|Default|GetPlayerPawn))
  ;[1 1 1] PAWN GAMEPAD MOVE
  (Networking|SwitchHasAuthority
    (:Authority
      _)
    (:Remote
      _))
  (if (> AxisValue 0.2)
    (Class|SPPawnCPP|SetRightKey _playerpawn true)
    (if (>= AxisValue 0.8)
      (Class|SPPawnCPP|SetSuperRightKey _playerpawn true)
      (else
        (Class|SPPawnCPP|SetSuperRightKey _playerpawn false)))
    (elif (< AxisValue -0.2)
      (Class|SPPawnCPP|SetLeftKey _playerpawn true)
      (if (<= AxisValue -0.8)
        (Class|SPPawnCPP|SetSuperLeftKey _playerpawn true)
        (else
          (Class|SPPawnCPP|SetSuperLeftKey _playerpawn false)))
      (else
        (Class|SPPawnCPP|SetRightKey _playerpawn false)
        (Class|SPPawnCPP|SetLeftKey _playerpawn false)
        (Class|SPPawnCPP|SetSuperLeftKey _playerpawn false)
        (Class|SPPawnCPP|SetSuperRightKey _playerpawn false)))))

(event Input|GamepadEvents|GamepadLeftY
  (params (AxisValue :type Float%20%28single-precision%29))
  (bind _playerpawn (Variables|Default|GetPlayerPawn))
  ;[1 1 1] PAWN GAMEPAD UP DOWN
  (Networking|SwitchHasAuthority
    (:Authority
      _)
    (:Remote
      _))
  (if (> AxisValue 0.0)
    (Class|SPPawnCPP|SetUpKey _playerpawn true)
    (elif (< AxisValue 0.0)
      (Class|SPPawnCPP|SetDownKey _playerpawn true)
      (else
        (Class|SPPawnCPP|SetUpKey _playerpawn false)
        (Class|SPPawnCPP|SetDownKey _playerpawn false)))))

(event Input|KeyboardEvents|AndroidBack
  (params (Key :type Key%20Structure :default "AnyKey"))
  ;[1 1 1] BACK
  (:Pressed
    (bind _outactors (Actor|GetAllActorsOfClass "/Game/BLUEPRINTS/WORLDSETTINGS/SPHUDBP.SPHUDBP_C"))
    (Default|ShowExit (Variables|/Game/BLUEPRINTS/HUD/SPMainHUD.SPMainHUD_C|GetInGameMenu_30 (Variables|/Game/BLUEPRINTS/WORLDSETTINGS/SPHUDBP.SPHUDBP_C|GetMainHUD (Utilities|Array|Get(acopy) _outactors))))))

(event Input|GamepadEvents|GamepadFaceButtonBottom
  (params (Key :type Key%20Structure :default "AnyKey"))
  ;[1 1 1] PAWN GAMEPAD CONTROL
)

(event Input|GamepadEvents|GamepadFaceButtonLeft
  (params (Key :type Key%20Structure :default "AnyKey"))
  ;[1 1 1] PAWN GAMEPAD CONTROL
)

(event Input|GamepadEvents|GamepadFaceButtonTop
  (params (Key :type Key%20Structure :default "AnyKey"))
  ;[1 1 1] PAWN GAMEPAD CONTROL
)

(event Input|GamepadEvents|GamepadFaceButtonRight
  (params (Key :type Key%20Structure :default "AnyKey"))
  ;[1 1 1] PAWN GAMEPAD CONTROL
)

(event Input|KeyboardEvents|Escape
  (params (Key :type Key%20Structure :default "AnyKey"))
  ;[1 1 1] BACK
  (:Pressed
    (bind _outactors (Actor|GetAllActorsOfClass "/Game/BLUEPRINTS/WORLDSETTINGS/SPHUDBP.SPHUDBP_C"))
    (Default|ShowExit (Variables|/Game/BLUEPRINTS/HUD/SPMainHUD.SPMainHUD_C|GetInGameMenu_30 (Variables|/Game/BLUEPRINTS/WORLDSETTINGS/SPHUDBP.SPHUDBP_C|GetMainHUD (Utilities|Array|Get(acopy) _outactors))))))

(fn ConstructionScript)

(fn NativeSpawnSPPawnBP
  (params (Location :type Vector) (Server :type Boolean))
  (Networking|SwitchHasAuthority
    (:Authority
      (if Server
        _
        (else
          _))
      (bind _returnvalue (Game|SpawnActorfromClass "/Game/BLUEPRINTS/WORLDSETTINGS/NinjaPawn.NinjaPawn_C" (Math|Conversions|ToTransform(Vector) Location) "AlwaysSpawn" 0 0))
      (return _returnvalue))
    (:Remote
      (return 0))))

(fn AxisPosition
  (return (Math|Vector2D|MakeVector2D (Class|Actor|GetInputAxisKeyValue) (Class|Actor|GetInputAxisKeyValue))))